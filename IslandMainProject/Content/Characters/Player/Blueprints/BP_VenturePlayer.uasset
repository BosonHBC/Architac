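; Player character Blueprint that adds vertical swim impulses, tool switching events, a pause menu and entry into building mode from exploration.
; On BeginPlay it creates the HUD, anchors the inventory slot window near the bottom centre and caches the planet actor.
; Inventory indicator events move the slot highlight and can return focus to the sending BlockSet window using copied relation data.
; Building mode requires a world grid and goes through the game mode and player controller.
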(event `InputAxis|SwimUpDown`
  (params (AxisValue :type "Float (single-precision)"))
  (bind _charactermovement (`self.CharacterMovement`))
  ;[1 1 1] Swim
  (if (`NavMovementComponent.IsSwimming` _charactermovement)
    (`CharacterMovementComponent.AddImpulse` _charactermovement (* (`KismetMathLibrary.MakeVector` 0.0 0.0 AxisValue) (0.0 0.0 25.0)) true)))

(event `self.ReceiveBeginPlay`
  (bind _returnvalue (`GameplayStatics.GetPlayerController` 0))
  (bind _inventorycomp (`self.InventoryComp`))
  (`|ExecutionSequence`
    (:`then_0`
      ;[1 1 1] Create Base UI HUD
      (bind _returnvalue_2 (`|CreateWidget` "/Game/UI/InventoryUI/BP_UI_HUD.BP_UI_HUD_C" _returnvalue))
      (bind _asbp_player_controller (cast `/Game/Base/BP_PlayerController` _returnvalue))
      (set `/Game/Base/BP_PlayerController.HUDWidget` _returnvalue_2 _asbp_player_controller)
      (`UserWidget.AddToViewport` _returnvalue_2 0))
    (:`then_1`
      ;[1 1 1] Create Inventory Slot
      (bind _returnvalue_3 (`InventoryComponent.GetNumOfSlots` _inventorycomp))
      (bind _returnvalue_4 (`|CreateWidget` "/Game/UI/InventoryUI/BP_UI_InventoryWindow.BP_UI_InventoryWindow_C" (`GameplayStatics.GetPlayerController` 0) _inventorycomp _returnvalue_3))
      (set `self.PlayerInventory` _returnvalue_4)
      (`UserWidget.AddToViewport` _returnvalue_4 0)
      (bind _asbp_player_controller_2 (cast `/Game/Base/BP_PlayerController` (`GameplayStatics.GetPlayerController` 0)))
      (bind _returnvalue_5 (`CanvasPanel.AddChildToCanvas` (`/Game/UI/InventoryUI/BP_UI_HUD.HudCanvas` (`/Game/Base/BP_PlayerController.HUDWidget` _asbp_player_controller_2)) _returnvalue_4))
      (`CanvasPanelSlot.SetAutoSize` _returnvalue_5 true)
      (`CanvasPanelSlot.SetAlignment` _returnvalue_5 (0.5 0.0))
      (`CanvasPanelSlot.SetAnchors` _returnvalue_5 (make `Anchors` (0.5 0.9) (0.5 0.9))))
    (:`then_2`
      ;[1 1 1] Get Planet Reference
      (bind _outactors (`GameplayStatics.GetAllActorsOfClass` "/Game/Environments/Terrain/Planet/BP_Planet.BP_Planet_C"))
      (set `self.PlanetRef` (`|GetArrayItem` _outactors)))))

(event `self.MoveUIIndicator`
  (params (direction :type "IntVector Structure") (istheoriginalwindow :type Boolean))
  (bind _playerinventory (`self.PlayerInventory`))
  (bind (_value _returnvalue) (`BlueprintMapLibrary.Map_Find` (`self.copyrelationdata`) (make `IntVector` 0)))
  ;[1 1 1] Move Indicator
  (if (not istheoriginalwindow)
    (bind (_updatedposition _isinthiswindow) (`/Game/UI/BasicUI/BP_BasicUI_Window.MoveSlotIndicator` _playerinventory direction))
    (if (not _isinthiswindow)
      (bind _returnvalue_2 (`self.GetKeyFromValueForRelationData` self))
      (bind (_x _y _z) (break `IntVector` _returnvalue_2))
      (bind (_x_2 _y_2 _z_2) (break `IntVector` _updatedposition))
      (if (and (== _x _x_2) (== _y _y_2) (== _z _z_2))
        (`/Game/UI/BasicUI/BP_BasicUI_Window.UnHighlightCurrentSlot` _playerinventory)
        (if _returnvalue
          (bind _asblock_set (cast `BlockSet` _value))
          (`BlockSet.FocusThisWindow` _asblock_set (`self.Sender`)))))))

(event `self.CloseWindow`
  ;[1 1 1] Open And Close Inventory Indicator
  (`/Game/UI/BasicUI/BP_BasicUI_Window.UnHighlightCurrentSlot` (`self.PlayerInventory`)))

(event `self.FocusThisWindow`
  (params (sender :type "Actor Object Reference"))
  ;[1 1 1] Focus This Window
  (set `self.Sender` sender)
  (`/Game/UI/BasicUI/BP_BasicUI_Window.SetUpInitialSlotPosition` (`self.PlayerInventory`))
  (bind _asblock_set (cast `BlockSet` sender))
  (set `self.copyrelationdata` (`BlockSet.copyrelationdata` _asblock_set)))

(event `self.OpenWindow`
  ;[1 1 1] Open And Close Inventory Indicator
  (`/Game/UI/BasicUI/BP_BasicUI_Window.UnHighlightCurrentSlot` (`self.PlayerInventory`)))

(event `self.BPSwitchToItem1`
  ;[1 1 1] Tool UI Indication
  (bind _asbp_player_controller (cast `/Game/Base/BP_PlayerController` (`GameplayStatics.GetPlayerController` 0)))
  (`/Game/Base/BP_PlayerController.SwitchItem1` _asbp_player_controller))

(event `InputAction|EnterBuildingMode`
  (params (Key :type "Key Structure"))
  ;[1 1 1] Go to building mode
  (:`Pressed`
    (if (`|EnumEquality` (`self.VenturePawnState`) "E_EXPLORE")
      (bind _asbp_game_mode (cast `/Game/Base/BP_GameMode` (`GameplayStatics.GetGameMode`)))
      (bind _outactors (`GameplayStatics.GetAllActorsOfClass` "/Game/Building/Blueprints/BP_WorldGrid.BP_WorldGrid_C"))
      (if (> (`KismetArrayLibrary.Array_Length` _outactors) 0)
        (`IslandMainProjectGameModeBase.GoToBuildingMode` _asbp_game_mode (`|GetArrayItem` _outactors))
        (bind _asbp_player_controller (cast `/Game/Base/BP_PlayerController` (`GameplayStatics.GetPlayerController` 0)))
        (`/Game/Base/BP_PlayerController.UI_TransitionToBuildingMode` _asbp_player_controller)
        (bind _asbp_game_mode_2 (cast `/Game/Base/BP_GameMode` (`GameplayStatics.GetGameMode`)))
        (`AudioManagerComponent.Play` (`/Game/Base/BP_GameMode.AudioManager` _asbp_game_mode_2) "UIBuildingOpen" (0.0 0.0 0.0))
        (else
          (`KismetSystemLibrary.PrintString` "No World Grid Defined" true true (struct :`R` 1.0 :`G` 0.08449 :`A` 1.0)))))))

(event `self.BPSwitchToItem2`
  ;[1 1 1] Tool UI Indication
  (bind _asbp_player_controller (cast `/Game/Base/BP_PlayerController` (`GameplayStatics.GetPlayerController` 0)))
  (`/Game/Base/BP_PlayerController.SwitchItem2` _asbp_player_controller))

(event `self.BPSwitchToItem3`
  ;[1 1 1] Tool UI Indication
  (bind _asbp_player_controller (cast `/Game/Base/BP_PlayerController` (`GameplayStatics.GetPlayerController` 0)))
  (`/Game/Base/BP_PlayerController.SwitchItem3` _asbp_player_controller))

(event `Key|Escape` :paused true
  (params (Key :type "Key Structure"))
  (bind _returnvalue (`GameplayStatics.GetPlayerController` 0))
  ;[1 1 1] Pause Menu
  (:`Pressed`
    (if (`GameplayStatics.IsGamePaused`)
      (set `PlayerController.bShowMouseCursor` false _returnvalue)
      (`GameplayStatics.SetGamePaused` false)
      (`Widget.RemoveFromParent` (stale _returnvalue_2))
      (`WidgetBlueprintLibrary.SetInputMode_GameOnly` _returnvalue)
      (else
        (set `PlayerController.bShowMouseCursor` true _returnvalue)
        (`GameplayStatics.SetGamePaused` true)
        (bind _returnvalue_2 (`|CreateWidget` "/Game/UI/PauseUI/PauseUI.PauseUI_C" _returnvalue))
        (`UserWidget.AddToViewport` _returnvalue_2 0)
        (`WidgetBlueprintLibrary.SetInputMode_GameAndUIEx` _returnvalue _returnvalue_2)))))

(fn `UserConstructionScript`)