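; BP_FatBird is a bird character Blueprint that passes movement, attack, damage and death state to its animation Blueprint, BP_BirdAnim.
; On BeginPlay it gives the anim instance references to itself and its BP_SkyAICtrl controller, then updates horizontal velocity every tick.
; Attack, damage and death events set anim flags.
; Damage also updates the widget health bar, and death hides it before destroying the actor after a delay.
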(event `self.ReceiveBeginPlay`
  ;[1 1 1] Init Anim BP Ref
  (bind _asbp_bird_anim (cast `/Game/Environments/Animals/BirdSmall/Animation/BP_BirdAnim` (`SkeletalMeshComponent.GetAnimInstance` (`self.SuperMesh`))))
  (set `/Game/Environments/Animals/BirdSmall/Animation/BP_BirdAnim.FatBirdRef` self _asbp_bird_anim)
  (bind _output_get (set `self.AnimBPRef` _asbp_bird_anim))
  (bind _asbp_sky_aictrl (cast `/Game/Environments/Animals/SkyCreatureAI/BP_SkyAICtrl` (`self.GetController`)))
  (set `/Game/Environments/Animals/BirdSmall/Animation/BP_BirdAnim.SkyAICtrlRef` _asbp_sky_aictrl _output_get))

(event `self.BPPerformAttack`
  (set `/Game/Environments/Animals/BirdSmall/Animation/BP_BirdAnim.bAttacking` true (`self.AnimBPRef`)))

(event `self.ReceiveTick`
  (params (DeltaSeconds :type "Float (single-precision)"))
  (set `/Game/Environments/Animals/BirdSmall/Animation/BP_BirdAnim.HorizontalVelocity` (`self.GetHorizontalVelocity`) (`self.AnimBPRef`)))

(event `self.BPOnGetdamage`
  (params (ratioOfHealth :type "Float (single-precision)"))
  ;[1 1 1] Get Dmg
  (`KismetSystemLibrary.PrintString` "Get damage")
  (bind _asui_damageable_health_bar (cast `/Game/Environments/Animals/BouncingFish/Blueprints/UI_DamageableHealthBar` (`WidgetComponent.GetUserWidgetObject` (`self.WidgetComp`))))
  (`ProgressBar.SetPercent` (`/Game/Environments/Animals/BouncingFish/Blueprints/UI_DamageableHealthBar.HealthBar` _asui_damageable_health_bar) ratioOfHealth)
  (set `/Game/Environments/Animals/BirdSmall/Animation/BP_BirdAnim.bGettingDamage` true (`self.AnimBPRef`)))

(event `self.BPDie`
  ;[1 1 1] Die
  (`SceneComponent.SetVisibility` (`self.WidgetComp`) false false)
  (set `/Game/Environments/Animals/BirdSmall/Animation/BP_BirdAnim.bDead` true (`self.AnimBPRef`))
  (`KismetSystemLibrary.Delay` 5.0)
  (`self.K2_DestroyActor`))

(fn `UserConstructionScript`)