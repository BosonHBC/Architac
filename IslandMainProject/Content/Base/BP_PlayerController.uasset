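; Player controller that builds the base HUD and manages on-screen control-tip widgets for walking, swimming and building.
; BeginPlay creates the tip widgets, then looping timers refresh a height readout from pawn Z and swap land or sea tips based on swimming.
; Transition functions swap player and building tips on the HUD canvas, with an input toggling extra building controls.
; SwitchItem events highlight the selected tool in the circle widget.
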(event `self.ReceiveBeginPlay`
  (bind _returnvalue (`GameplayStatics.GetPlayerController` 0))
  (set `self.PressH` false)
  ;[1 1 1] Create Base UI HUD
  (bind _returnvalue_2 (`|CreateWidget` "/Game/UI/InventoryUI/BP_UI_HUD.BP_UI_HUD_C" _returnvalue))
  (bind _asbp_player_controller (cast `/Game/Base/BP_PlayerController` _returnvalue))
  (set `/Game/Base/BP_PlayerController.HUDWidget` _returnvalue_2 _asbp_player_controller)
  (`UserWidget.AddToViewport` _returnvalue_2 0)
  ;[1 1 1] Building Tip H
  (bind _returnvalue_3 (`|CreateWidget` "/Game/UI/TipsUI/BP_UI_TIPS_BuidlingHKey.BP_UI_TIPS_BuidlingHKey_C" self))
  (set `self.BuildingTipsUI` _returnvalue_3)
  (bind _returnvalue_4 (`|CreateWidget` "/Game/UI/TipsUI/BP_UI_TIPS_BuidlingControlTips.BP_UI_TIPS_BuidlingControlTips_C" self))
  (set `self.BuildingTipsH` _returnvalue_4)
  ;[1 1 1] Tip Circle
  (bind _returnvalue_5 (`|CreateWidget` "/Game/UI/TipsUI/BP_UI_TIPS_CircleTools.BP_UI_TIPS_CircleTools_C" self))
  (set `self.circleTips` _returnvalue_5)
  (`UserWidget.AddToViewport` _returnvalue_5 0)
  (bind _returnvalue_6 (`CanvasPanel.AddChildToCanvas` (`/Game/UI/InventoryUI/BP_UI_HUD.HudCanvas` (`self.HUDWidget`)) _returnvalue_5))
  (`CanvasPanelSlot.SetAnchors` _returnvalue_6 (make `Anchors` (0.02 0.8) (0.02 0.8)))
  ;[1 1 1] Player Height level
  (bind _returnvalue_7 (`|CreateWidget` "/Game/UI/TipsUI/BP_UI_TIPS_CurrentHeight.BP_UI_TIPS_CurrentHeight_C" self))
  (set `self.UI_PlayerHeight` _returnvalue_7)
  (`UserWidget.AddToViewport` _returnvalue_7 0)
  (bind _returnvalue_8 (`CanvasPanel.AddChildToCanvas` (`/Game/UI/InventoryUI/BP_UI_HUD.HudCanvas` (`self.HUDWidget`)) _returnvalue_7))
  (`CanvasPanelSlot.SetAnchors` _returnvalue_8 (make `Anchors` (0.85 0.01) (0.85 0.01)))
  ;[1 1 1] Building Mode Level
  (bind _returnvalue_9 (`|CreateWidget` "/Game/UI/TipsUI/BP_UI_TIPS_BuildingModeB.BP_UI_TIPS_BuildingModeB_C" self))
  (bind _output_get (set `self.BuildingModeB` _returnvalue_9))
  (`UserWidget.AddToViewport` _returnvalue_9 0)
  (`UserWidget.AddToViewport` _output_get 0)
  (bind _returnvalue_10 (`CanvasPanel.AddChildToCanvas` (`/Game/UI/InventoryUI/BP_UI_HUD.HudCanvas` (`self.HUDWidget`)) _returnvalue_9))
  (`CanvasPanelSlot.SetAnchors` _returnvalue_10 (make `Anchors` (0.0 0.0)))
  ;[1 1 1] Sea state
  (bind _returnvalue_11 (`|CreateWidget` "/Game/UI/TipsUI/BP_UI_TIPS_SeaMove.BP_UI_TIPS_SeaMove_C" self))
  (set `self.SeaStateUI` _returnvalue_11)
  ;[1 1 1] Land state
  (bind _returnvalue_12 (`|CreateWidget` "/Game/UI/TipsUI/BP_UI_TIPS_LandMove.BP_UI_TIPS_LandMove_C" self))
  (set `self.LandStateUI` _returnvalue_12)
  (`KismetSystemLibrary.K2_SetTimer` self "UpdatePlayerHeight" 1.5 true)
  (`KismetSystemLibrary.K2_SetTimer` self "UpdateControllerTipState" 1.5 true))

(event `SwitchItem1`
  (bind _circletips (`self.circleTips`))
  (bind _image01 (`/Game/UI/TipsUI/BP_UI_TIPS_CircleTools.Image01` _circletips))
  (bind _image03 (`/Game/UI/TipsUI/BP_UI_TIPS_CircleTools.Image03` _circletips))
  (bind _image02 (`/Game/UI/TipsUI/BP_UI_TIPS_CircleTools.Image02` _circletips))
  ;[1 1 1] Tool UI Tips Animation
  (`Image.SetColorAndOpacity` _image01 (struct :`R` 1.0 :`G` 0.8 :`A` 1.0))
  (`Image.SetColorAndOpacity` _image02 (struct :`R` 1.0 :`G` 1.0 :`B` 1.0 :`A` 1.0))
  (`Image.SetColorAndOpacity` _image03 (struct :`R` 1.0 :`G` 1.0 :`B` 1.0 :`A` 1.0))
  (`Widget.SetRenderScale` _image01 (1.1 1.1))
  (`Widget.SetRenderScale` _image02 (1.0 1.0))
  (`Widget.SetRenderScale` _image03 (1.0 1.0))
  (`Widget.SetRenderScale` (`/Game/UI/TipsUI/BP_UI_TIPS_CircleTools.Tool01` _circletips) (1.6 1.6))
  (`Widget.SetRenderScale` (`/Game/UI/TipsUI/BP_UI_TIPS_CircleTools.Tool02` _circletips) (1.0 1.0)))

(event `SwitchItem2`
  (bind _circletips (`self.circleTips`))
  (bind _image03 (`/Game/UI/TipsUI/BP_UI_TIPS_CircleTools.Image03` _circletips))
  (bind _image01 (`/Game/UI/TipsUI/BP_UI_TIPS_CircleTools.Image01` _circletips))
  (bind _image02 (`/Game/UI/TipsUI/BP_UI_TIPS_CircleTools.Image02` _circletips))
  ;[1 1 1] Tool UI Tips Animation
  (`Image.SetColorAndOpacity` _image02 (struct :`R` 1.0 :`G` 0.8 :`A` 1.0))
  (`Image.SetColorAndOpacity` _image01 (struct :`R` 1.0 :`G` 1.0 :`B` 1.0 :`A` 1.0))
  (`Image.SetColorAndOpacity` _image03 (struct :`R` 1.0 :`G` 1.0 :`B` 1.0 :`A` 1.0))
  (`Widget.SetRenderScale` _image02 (1.1 1.1))
  (`Widget.SetRenderScale` _image01 (1.0 1.0))
  (`Widget.SetRenderScale` _image03 (1.0 1.0))
  (`Widget.SetRenderScale` (`/Game/UI/TipsUI/BP_UI_TIPS_CircleTools.Tool02` _circletips) (1.6 1.6))
  (`Widget.SetRenderScale` (`/Game/UI/TipsUI/BP_UI_TIPS_CircleTools.Tool01` _circletips) (1.0 1.0)))

(event `SwitchItem3`
  (bind _circletips (`self.circleTips`))
  (bind _image02 (`/Game/UI/TipsUI/BP_UI_TIPS_CircleTools.Image02` _circletips))
  (bind _image03 (`/Game/UI/TipsUI/BP_UI_TIPS_CircleTools.Image03` _circletips))
  (bind _image01 (`/Game/UI/TipsUI/BP_UI_TIPS_CircleTools.Image01` _circletips))
  ;[1 1 1] Tool UI Tips Animation
  (`Image.SetColorAndOpacity` _image03 (struct :`R` 1.0 :`G` 0.8 :`A` 1.0))
  (`Image.SetColorAndOpacity` _image02 (struct :`R` 1.0 :`G` 1.0 :`B` 1.0 :`A` 1.0))
  (`Image.SetColorAndOpacity` _image01 (struct :`R` 1.0 :`G` 1.0 :`B` 1.0 :`A` 1.0))
  (`Widget.SetRenderScale` _image03 (1.0 1.0))
  (`Widget.SetRenderScale` _image02 (1.0 1.0))
  (`Widget.SetRenderScale` _image01 (1.0 1.0))
  (`Widget.SetRenderScale` (`/Game/UI/TipsUI/BP_UI_TIPS_CircleTools.Tool02` _circletips) (1.0 1.0))
  (`Widget.SetRenderScale` (`/Game/UI/TipsUI/BP_UI_TIPS_CircleTools.Tool01` _circletips) (1.0 1.0)))

(event `InputAction|BuilldingControlTips`
  (params (Key :type "Key Structure"))
  (bind _buildingtipsh (`self.BuildingTipsH`))
  ;[1 1 1] BuildingContolTips_PressH
  (:`Pressed`
    (if (`self.isBuildingMode`)
      (`self.SetPressH`)
      (if (`self.PressH`)
        (bind _returnvalue (`CanvasPanel.AddChildToCanvas` (`/Game/UI/InventoryUI/BP_UI_HUD.HudCanvas` (`self.HUDWidget`)) _buildingtipsh))
        (`CanvasPanelSlot.SetAnchors` _returnvalue (make `Anchors` (0.3 0.0) (0.3 0.0)))
        (else
          (`Widget.RemoveFromParent` _buildingtipsh))))))

(fn `SetPressH`
  (if (`self.PressH`)
    (set `self.PressH` false)
    (else
      (set `self.PressH` true))))

(fn `UI_TransitionToBuildingMode`
  (`Widget.RemoveFromParent` (`self.circleTips`))
  (`Widget.RemoveFromParent` (`self.BuildingModeB`))
  (`Widget.RemoveFromParent` (`self.LandStateUI`))
  (bind _returnvalue (`CanvasPanel.AddChildToCanvas` (`/Game/UI/InventoryUI/BP_UI_HUD.HudCanvas` (`self.HUDWidget`)) (`self.BuildingTipsUI`)))
  (`CanvasPanelSlot.SetAnchors` _returnvalue (make `Anchors` (0.0 0.0)))
  (set `self.isBuildingMode` true)
  (set `self.PressH` false))

(fn `UI_TransitionToPlayerMode`
  (bind _returnvalue (`CanvasPanel.AddChildToCanvas` (`/Game/UI/InventoryUI/BP_UI_HUD.HudCanvas` (`self.HUDWidget`)) (`self.circleTips`)))
  (`CanvasPanelSlot.SetAnchors` _returnvalue (make `Anchors` (0.02 0.8) (0.02 0.8)))
  (bind _returnvalue_2 (`CanvasPanel.AddChildToCanvas` (`/Game/UI/InventoryUI/BP_UI_HUD.HudCanvas` (`self.HUDWidget`)) (`self.BuildingModeB`)))
  (`CanvasPanelSlot.SetAnchors` _returnvalue_2 (make `Anchors` (0.0 0.0)))
  (bind _returnvalue_3 (`CanvasPanel.AddChildToCanvas` (`/Game/UI/InventoryUI/BP_UI_HUD.HudCanvas` (`self.HUDWidget`)) (`self.LandStateUI`)))
  (`CanvasPanelSlot.SetAnchors` _returnvalue_3 (make `Anchors` (0.75 0.95) (0.75 0.95)))
  (`Widget.RemoveFromParent` (`self.BuildingTipsUI`))
  (`Widget.RemoveFromParent` (`self.BuildingTipsH`))
  (set `self.isBuildingMode` false))

(fn `UpdateControllerTipState`
  (bind _asventure_pawn (cast `VenturePawn` (`GameplayStatics.GetPlayerPawn` 0)))
  (if (`NavMovementComponent.IsSwimming` (`Character.CharacterMovement` _asventure_pawn))
    ;[1 1 1] SeaMoveTips
    (bind _returnvalue (`CanvasPanel.AddChildToCanvas` (`/Game/UI/InventoryUI/BP_UI_HUD.HudCanvas` (`self.HUDWidget`)) (`self.SeaStateUI`)))
    (`CanvasPanelSlot.SetAnchors` _returnvalue (make `Anchors` (0.75 0.95) (0.75 0.95)))
    (`Widget.RemoveFromParent` (`self.LandStateUI`))
    (else
      ;[1 1 1] LandMoveTips
      (bind _returnvalue_2 (`CanvasPanel.AddChildToCanvas` (`/Game/UI/InventoryUI/BP_UI_HUD.HudCanvas` (`self.HUDWidget`)) (`self.LandStateUI`)))
      (`CanvasPanelSlot.SetAnchors` _returnvalue_2 (make `Anchors` (0.78 0.93) (0.78 0.93)))
      (`Widget.RemoveFromParent` (`self.SeaStateUI`)))))

(fn `UpdatePlayerHeight`
  (`TextBlock.SetText` (`/Game/UI/TipsUI/BP_UI_TIPS_CurrentHeight.PlayerHeight` (`self.UI_PlayerHeight`)) (`KismetTextLibrary.Conv_IntToText` (`KismetMathLibrary.Round` (/ (.z (`self.K2_GetActorLocation` (`GameplayStatics.GetPlayerPawn` 0))) 200.0)))))

(fn `UserConstructionScript`)