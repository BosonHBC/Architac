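; BP_OctopusMinions is a small octopus minion that reacts visually to attacking, taking damage and dying.
; BeginPlay caches its BP_OctopusSmallAnimBP, and the attack, damage and death events set flags on that AnimBP to drive animation.
; Damage also updates the widget health bar from the passed health ratio.
; Death hides the widget and destroys the actor after a short delay.
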(event `self.ReceiveBeginPlay`
  ;[1 1 1] Set AnimBP
  (bind _asbp_octopus_small_anim_bp (cast `/Game/Environments/Animals/OctopusSmall/Animation/BP_OctopusSmallAnimBP` (`SkeletalMeshComponent.GetAnimInstance` (`self.SuperMesh`))))
  (set `self.OctopusMinonAnimBP` _asbp_octopus_small_anim_bp))

(event `self.BPPerformAttack`
  ;[1 1 1] Attack
  (set `/Game/Environments/Animals/OctopusSmall/Animation/BP_OctopusSmallAnimBP.bAttacking` true (`self.OctopusMinonAnimBP`)))

(event `self.BPOnGetdamage`
  (params (ratioOfHealth :type "Float (single-precision)"))
  ;[1 1 1] SetUI
  (`KismetSystemLibrary.PrintString` "Get damage")
  (bind _asui_damageable_health_bar (cast `/Game/Environments/Animals/BouncingFish/Blueprints/UI_DamageableHealthBar` (`WidgetComponent.GetUserWidgetObject` (`self.WidgetComp`))))
  (`ProgressBar.SetPercent` (`/Game/Environments/Animals/BouncingFish/Blueprints/UI_DamageableHealthBar.HealthBar` _asui_damageable_health_bar) ratioOfHealth)
  ;[1 1 1] Update Animation
  (bind _asbp_octopus_small_anim_bp (cast `/Game/Environments/Animals/OctopusSmall/Animation/BP_OctopusSmallAnimBP` (`SkeletalMeshComponent.GetAnimInstance` (`self.SuperMesh`))))
  (set `/Game/Environments/Animals/OctopusSmall/Animation/BP_OctopusSmallAnimBP.bGettingDamage` true _asbp_octopus_small_anim_bp))

(event `self.BPDie`
  ;[1 1 1] Disable UI
  (`SceneComponent.SetVisibility` (`self.WidgetComp`) false false)
  ;[1 1 1] Update Animation
  (set `/Game/Environments/Animals/OctopusSmall/Animation/BP_OctopusSmallAnimBP.bDead` true (`self.OctopusMinonAnimBP`))
  ;[1 1 1] DelayDestroy
  (`KismetSystemLibrary.Delay` 5.0)
  (`self.K2_DestroyActor`))

(fn `UserConstructionScript`)