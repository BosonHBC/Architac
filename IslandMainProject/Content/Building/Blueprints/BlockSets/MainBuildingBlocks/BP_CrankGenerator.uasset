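; BP_CrankGenerator is a crank generator building block that switches its generator on and off.
; GeneratorStart and GeneratorStop set the GeneratorActive flag and drive one shared timeline, reversed on start and played forward on stop.
; The timeline's GeneratorPlayRate track feeds SKGenerator's play rate, so a single curve handles both animation transitions.
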(event `Generator Stop`
  (set `self.Generator Active` false)
  (bind (_direction _generatorplayrate) (`Timeline|GeneratorStartStop_Timeline` :!label _label)
    (:`Update`
      (`SkeletalMeshComponent.SetPlayRate` (`self.SK_Generator`) _generatorplayrate))))

(event `Generator Start`
  (set `self.Generator Active` true)
  (goto _label :!via `Reverse`))

(fn `UserConstructionScript`
  (`parent.UserConstructionScript`))