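; BP_GameProgressDirector is a director Blueprint that bootstraps spawn services when play begins.
; On BeginPlay it spawns monster and pickup spawn service actors at the world origin and stores references to both.
; It then has the monster spawner mass-spawn the SpawnMonsterList at a small X offset from player 0's pawn location.
; The pickup spawner is only created and stored here.
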(event `self.ReceiveBeginPlay`
  (bind _returnvalue (`|SpawnActorFromClass` "/Game/Base/Services/BP_MonsterSpawnServiceActor.BP_MonsterSpawnServiceActor_C" (`KismetMathLibrary.MakeTransform` (0.0 0.0 0.0)) "Undefined" "OverrideRootScale" null null))
  (`self.SetMonsterSpawner` _returnvalue)
  (bind _returnvalue_2 (`|SpawnActorFromClass` "/Game/Base/Services/BP_PickSpawnServiceActor.BP_PickSpawnServiceActor_C" (`KismetMathLibrary.MakeTransform` (0.0 0.0 0.0)) "Undefined" "OverrideRootScale" null null))
  (`self.SetPickupSpawner` _returnvalue_2)
  (bind _returnvalue_3 (`self.GetMonsterSpawner`))
  (`MonsterSpawnServiceActor.MassSpawning` _returnvalue_3 (`self.SpawnMonsterList`) (+ (`self.K2_GetActorLocation` (`GameplayStatics.GetPlayerPawn` 0)) (`KismetMathLibrary.MakeVector` 2.0))))

(fn `UserConstructionScript`)