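; Widget component for the building system that shows an indicator icon through a UI_IndicatorWidget.
; Every tick it fetches a texture with GetTexture and pushes it to the widget, with no change check.
; Helpers wrap a texture or material in a 32x32 brush for SetImage, which passes it to the widget.
; ClearImage clears all images on the widget.
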(event `self.ReceiveTick`
  (params (DeltaSeconds :type "Float (single-precision)"))
  (`self.SetImageByTexture` (`self.GetTexture`)))

(fn `ClearImage`
  (bind _asui_indicator_widget (cast `/Game/UI/BuildingUI/UI_IndicatorWidget` (`self.GetUserWidgetObject`)))
  (`/Game/UI/BuildingUI/UI_IndicatorWidget.ClearAllImage` _asui_indicator_widget))

(fn `SetImage`
  (params (IndicatorImage :type "SlateBrush Structure"))
  (bind _asui_indicator_widget (cast `/Game/UI/BuildingUI/UI_IndicatorWidget` (`self.GetUserWidgetObject`)))
  (`/Game/UI/BuildingUI/UI_IndicatorWidget.SetCurrentImage` _asui_indicator_widget IndicatorImage))

(fn `SetImageByMaterial`
  (params (mat :type "Material Object Reference"))
  (`self.SetImage` (`WidgetBlueprintLibrary.MakeBrushFromMaterial` mat)))

(fn `SetImageByTexture`
  (params (texture :type "Texture Object Reference"))
  (`self.SetImage` (make `SlateBrush` (32.0 32.0) (struct) (struct :`SpecifiedColor` (struct :`R` 1.0 :`G` 1.0 :`B` 1.0 :`A` 1.0) :`ColorUseRule` "UseColor_Specified") texture)))