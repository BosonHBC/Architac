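; BP_Factory is a factory building block that links to a nearby warehouse and passes its inventory on to it.
; BeginPlay scans building blocks in range, and UpdateWareHouse keeps the closest warehouse; a similar resource scan casts to BP_Resource but does nothing further.
; Tick moves the factory inventory into the connected warehouse every frame.
; OpenWindow instead throws out all items and sets the player's VenturePawn to explore state.
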(event `self.ReceiveBeginPlay`
  (`parent.ReceiveBeginPlay`)
  (`|ExecutionSequence`
    (:`then_0`
      ;[1 1 1] WarehouseConnection
      (bind _result (`BlueprintSetLibrary.Set_ToArray` (`self.GetBuildingBlockSetInDistance` (`self.WareHouseConnectionDistance`))))
      (for _array_element _result
        (bind _asbp_warehouse (cast `/Game/Building/Blueprints/BlockSets/MainBuildingBlocks/BP_Warehouse` _array_element))
        (`self.UpdateWareHouse` _asbp_warehouse)))
    (:`then_1`
      ;[1 1 1] ResourceConnection
      (bind _result_2 (`BlueprintSetLibrary.Set_ToArray` (`self.GetBuildingBlockSetInDistance` (`self.ResourceConnectionDistance`))))
      (for _array_element_2 _result_2
        (cast `/Game/Building/Blueprints/BlockSets/MainBuildingBlocks/BP_Resource` _array_element_2)))))

(event `self.ReceiveTick`
  (params (DeltaSeconds :type "Float (single-precision)"))
  (bind _connectedwarehouse (`self.ConnectedWareHouse`))
  ;[1 1 1] Transfering resources
  (`parent.ReceiveTick` DeltaSeconds)
  (`/Engine/EditorBlueprintResources/StandardMacros.IsValid` _connectedwarehouse
    (:`Is Valid`
      (`InventoryUtility.MoveInventoryToAnother` (`self.Inventory`) (`/Game/Building/Blueprints/BlockSets/MainBuildingBlocks/BP_Warehouse.Inventory` _connectedwarehouse)))))

(event `self.OpenWindow`
  (`InventoryComponent.ThrowAllItemsInDirection` (`self.Inventory`) (0.0 0.0 0.0))
  (bind _asventure_pawn (cast `VenturePawn` (`GameplayStatics.GetPlayerPawn` 0)))
  (set `VenturePawn.VenturePawnState` "E_EXPLORE" _asventure_pawn))

(fn `UpdateWareHouse`
  (params (UpdateWareHouse :type "/Game/Building/Blueprints/BlockSets/MainBuildingBlocks/BP_Warehouse Object Reference"))
  (bind _connectedwarehouse (`self.ConnectedWareHouse`))
  (`/Engine/EditorBlueprintResources/StandardMacros.IsValid` _connectedwarehouse
    (:`Is Valid`
      (if (< (`KismetMathLibrary.Vector_Distance` (`self.K2_GetActorLocation`) (`self.K2_GetActorLocation` UpdateWareHouse)) (`KismetMathLibrary.Vector_Distance` (`self.K2_GetActorLocation`) (`self.K2_GetActorLocation` _connectedwarehouse)))
        (set `self.ConnectedWareHouse` UpdateWareHouse :!label _label)))
    (:`Is Not Valid`
      (goto _label))))

(fn `UserConstructionScript`
  (`parent.UserConstructionScript`))