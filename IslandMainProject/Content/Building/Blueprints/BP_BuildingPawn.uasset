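; Building-mode pawn Blueprint that serves as the UI bridge for selecting block sets to build.
; It creates a building window widget and forwards show, hide, option loading and directional navigation events to it, playing sounds via the game mode's AudioManager.
; Highlight changes load the selected block set, and confirming enters placement mode if resource requirements pass.
; The exit input returns the game mode and player controller UI to exploration.
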(event `self.ReceiveBeginPlay`
  ;[1 1 1] Add Building Window To Viewport
  (`|ExecutionSequence`
    (:`then_0`
      (bind _returnvalue (`|CreateWidget` "/Game/UI/BuildingUI/BuildingUILeft/BP_UI_BuildingWindow.BP_UI_BuildingWindow_C" (`GameplayStatics.GetPlayerController` 0)))
      (bind _output_get (set `self.BuildingWindow` _returnvalue))
      (`UserWidget.AddToViewport` _returnvalue 0)
      (`UserWidget.SetAnchorsInViewport` _returnvalue (make `Anchors` (0.0 0.08) (0.0 0.08)))
      (`/Game/UI/BuildingUI/BuildingUILeft/BP_UI_BuildingWindow.HideWindow` _output_get)
      (add `/Game/UI/BuildingUI/BuildingUILeft/BP_UI_BuildingWindow.OnChangedOption` (`self.BuildingWindow`) (delegate `OnChangedOption`)))
    (:`then_1`
      (bind _asbp_game_mode (cast `/Game/Base/BP_GameMode` (`GameplayStatics.GetGameMode`)))
      (set `self.AudioManager` (`/Game/Base/BP_GameMode.AudioManager` _asbp_game_mode)))))

(event `InputAction|ExitBuildingMode`
  (params (Key :type "Key Structure"))
  (bind _audiomanager (`self.AudioManager`))
  ;[1 1 1] Go to venture mode
  (:`Pressed`
    (bind _asbp_game_mode (cast `/Game/Base/BP_GameMode` (`GameplayStatics.GetGameMode`)))
    (`IslandMainProjectGameModeBase.GoToExploreMode` _asbp_game_mode)
    (bind _asbp_player_controller (cast `/Game/Base/BP_PlayerController` (`GameplayStatics.GetPlayerController` 0)))
    (`/Game/Base/BP_PlayerController.UI_TransitionToPlayerMode` _asbp_player_controller)
    (`/Engine/EditorBlueprintResources/StandardMacros.IsValid` _audiomanager
      (:`Is Valid`
        (`AudioManagerComponent.Play` _audiomanager "UIBuildingClose" (0.0 0.0 0.0))))))

(event `self.UIShowSelectionMenu`
  ;[1 1 1] Building UI Interface With Code
  (`/Game/UI/BuildingUI/BuildingUILeft/BP_UI_BuildingWindow.ShowWindow` (`self.BuildingWindow`)))

(event `self.UIHideSelectionMenu`
  ;[1 1 1] Building UI Interface With Code
  (`/Game/UI/BuildingUI/BuildingUILeft/BP_UI_BuildingWindow.HideWindow` (`self.BuildingWindow`)))

(event `self.UIChangeBlockSetLeft`
  (bind _audiomanager (`self.AudioManager`))
  ;[1 1 1] Building UI Interface With Code
  (`/Game/UI/BuildingUI/BuildingUILeft/BP_UI_BuildingWindow.MoveOption` (`self.BuildingWindow`) (make `IntVector` -1))
  (`/Engine/EditorBlueprintResources/StandardMacros.IsValid` _audiomanager :!label _label
    (:`Is Valid`
      (`AudioManagerComponent.Play` _audiomanager "UIBuildingNavigation" (0.0 0.0 0.0)))))

(event `self.UIChangeBlockSetRight`
  ;[1 1 1] Building UI Interface With Code
  (`/Game/UI/BuildingUI/BuildingUILeft/BP_UI_BuildingWindow.MoveOption` (`self.BuildingWindow`) (make `IntVector` 1))
  (goto _label))

(event `self.UIChangeBlockSetDown`
  ;[1 1 1] Building UI Interface With Code
  (`/Game/UI/BuildingUI/BuildingUILeft/BP_UI_BuildingWindow.MoveOption` (`self.BuildingWindow`) (make `IntVector` 0 -1))
  (goto _label))

(event `self.UIChangeBlockSetUp`
  ;[1 1 1] Building UI Interface With Code
  (`/Game/UI/BuildingUI/BuildingUILeft/BP_UI_BuildingWindow.MoveOption` (`self.BuildingWindow`) (make `IntVector` 0 1))
  (goto _label))

(event `self.UILoadBlockSetOptions`
  (params (options :type "Array of BlockSetData Structure (by ref)") (inventory :type "InventoryComponent Object Reference"))
  ;[1 1 1] Building UI Interface With Code
  (`/Game/UI/BuildingUI/BuildingUILeft/BP_UI_BuildingWindow.LoadOptions` (`self.BuildingWindow`) options inventory))

(event `OnChangedOption`
  ;[1 1 1] Building UI Interface With Code
  (bind _highlightedblocksetclass (`/Game/UI/BuildingUI/BuildingUILeft/BP_UI_BuildingWindow.GetCurrentlyHighlightedBlockSet` (`self.BuildingWindow`)))
  (`self.UIOnLoadSelectedBlockSet` _highlightedblocksetclass))

(event `self.UIConfirmBlockSetSelection`
  ;[1 1 1] Building UI Interface With Code
  (bind _highlightedblocksetclass (`/Game/UI/BuildingUI/BuildingUILeft/BP_UI_BuildingWindow.GetCurrentlyHighlightedBlockSet` (`self.BuildingWindow`)))
  (bind _returnvalue (`self.ConfirmResourceRequirements` _highlightedblocksetclass))
  (if _returnvalue
    (`self.GoToPlacementMode`)))

(fn `UserConstructionScript`)