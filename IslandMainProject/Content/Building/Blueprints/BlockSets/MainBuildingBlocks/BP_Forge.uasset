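; Forge building block that converts one resource into another through an interactive UI window.
; On BeginPlay it reads the ResourceConversion component's rate and first input/output item rows to create the window, printing an error for missing rows.
; Interaction calls ConvertItem immediately if input is available, then runs a one-second Delay loop as a countdown.
; CanProcessNextAction blocks opening, converting and closing until the countdown ends.
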(event `self.ReceiveBeginPlay`
  (bind (_inputitems _outputitems _rateinseconds) (break `ConversionPropertiesRow` (`ResourceConversionComponent.GetConversionPropertiesData` (`self.ResourceConversion`))))
  (bind (_itemrow _amount) (break `ItemAmount` (`|GetArrayItem` (`.ItemAmounts` (break `ItemAmountGroup` _inputitems)))))
  (bind (_itemrow_2 _amount_2) (break `ItemAmount` (`|GetArrayItem` (`.ItemAmounts` (break `ItemAmountGroup` _outputitems)))))
  (bind (_datatable _rowname) (break `DataTableRowHandle` _itemrow))
  (bind (_datatable_2 _rowname_2) (break `DataTableRowHandle` _itemrow_2))
  ;[1 1 1] Set data for UI
  (set `self.ConversionTime` _rateinseconds)
  (bind _returnvalue (`|GetDataTableRow` _datatable _rowname)
    (:`then`
      (bind _returnvalue_2 (`|GetDataTableRow` _datatable_2 _rowname_2)
        (:`then`
          (set `self.ResourceInput` _returnvalue)
          (set `self.ResourceOutput` _returnvalue_2)
          (set `self.InputResourceAmount` _amount)
          (set `self.OutputResourceAmount` _amount_2)
          ;[1 1 1] SetUp Window
          (bind _returnvalue_3 (`|CreateWidget` "/Game/UI/ForgeUI/BP_UI_ForgeWindow.BP_UI_ForgeWindow_C" (`GameplayStatics.GetPlayerController` 0) null (`self.ConversionTime`)))
          (set `self.UIForgeWindow` _returnvalue_3)
          ;[1 1 1] Set Intaractable Indication
          (`/Game/Building/Blueprints/Components/BP_UI_IndicatorComponent.SetImageByTexture` (`self.Indicator_Tip_UI`) "/Game/UI/Images/BuildingDamageBG.BuildingDamageBG"))
        (:`RowNotFound`
          ;[1 1 1] Error Checking
          (set `self.FailedRowName` (`KismetStringLibrary.Conv_NameToString` _rowname_2))
          (set `self.FailedTablePath` (`KismetSystemLibrary.GetPathName` null))
          (`KismetSystemLibrary.PrintString` (`KismetStringLibrary.Concat_StrStr` "Row <" (`self.FailedRowName`) "> For Data Table <" (`self.FailedTablePath`) "> Not Found") true true (struct :`R` 1.0 :`A` 1.0) 10.0 :!label _label))))
    (:`RowNotFound`
      (set `self.FailedRowName` (`KismetStringLibrary.Conv_NameToString` _rowname))
      (set `self.FailedTablePath` (`KismetSystemLibrary.GetPathName` null))
      (goto _label))))

(event `self.OpenWindow`
  (bind (_itemid _itempickup _name _action _amount _maxstack _thumbnail) (break `InventoryItem` (`self.ResourceInput`)))
  (bind (_itemid_2 _itempickup_2 _name_2 _action_2 _amount_2 _maxstack_2 _thumbnail_2) (break `InventoryItem` (`self.ResourceOutput`)))
  ;[1 1 1] Open UI window
  (if (`self.CanProcessNextAction`)
    (set `self.CanProcessNextAction` false)
    (`UserWidget.AddToViewport` (`self.UIForgeWindow`) 0)
    (`UserWidget.SetAnchorsInViewport` (`self.UIForgeWindow`) (make `Anchors` (0.35 0.5) (0.35 0.5)))
    (bind _returnvalue (`ResourceConversionComponent.IsInputResourceAvailable` (`self.ResourceConversion`)))
    (`/Game/UI/ForgeUI/BP_UI_ForgeWindow.SetWindowInfo` (`self.UIForgeWindow`) _itemid (`self.InputResourceAmount`) _thumbnail _itemid_2 (`self.OutputResourceAmount`) _thumbnail_2 _returnvalue)
    (set `self.JustOpenTheWindow` 0)
    (`Image.SetBrushFromTexture` (`/Game/UI/ForgeUI/BP_UI_ForgeWindow.StartButton` (`self.UIForgeWindow`)) "/Game/UI/Images/ConverterStart.ConverterStart" false)
    (set `self.CanProcessNextAction` true)))

(event `self.InteractWithUI`
  ;[1 1 1] UI Interaction
  (`|ExecutionSequence`
    (:`then_0`
      (if (`self.CanProcessNextAction`)
        (bind _returnvalue (`ResourceConversionComponent.IsInputResourceAvailable` (`self.ResourceConversion`)))
        (if _returnvalue
          (`ResourceConversionComponent.ConvertItem` (`self.ResourceConversion`) 0)
          (`Image.SetBrushFromTexture` (`/Game/UI/ForgeUI/BP_UI_ForgeWindow.StartButton` (`self.UIForgeWindow`)) "/Game/UI/Images/ConverterButtonBg.ConverterButtonBg" false)
          (set `self.CanProcessNextAction` false)
          (set `self.Timer` (`KismetMathLibrary.FTrunc` (`/Game/UI/ForgeUI/BP_UI_ForgeWindow.ConvertTime` (`self.UIForgeWindow`))))
          (`KismetSystemLibrary.PrintString` "Hello" :!label _label_2)
          (`TextBlock.SetText` (`/Game/UI/ForgeUI/BP_UI_ForgeWindow.TimerText` (`self.UIForgeWindow`)) (`KismetTextLibrary.Conv_IntToText` (`self.Timer`)))
          (`KismetSystemLibrary.Delay` 1.0)
          (bind _output_get (set `self.Timer` (- (`self.Timer`) 1)))
          (if (!= _output_get 0)
            (goto _label_2)
            (else
              (`TextBlock.SetText` (`/Game/UI/ForgeUI/BP_UI_ForgeWindow.TimerText` (`self.UIForgeWindow`)) "")
              (`Image.SetBrushFromTexture` (`/Game/UI/ForgeUI/BP_UI_ForgeWindow.StartButton` (`self.UIForgeWindow`)) "/Game/UI/Images/ConverterStart.ConverterStart" false)
              (set `self.CanProcessNextAction` true))))))))

(event `self.CloseWindow`
  ;[1 1 1] Close window
  (if (`self.CanProcessNextAction`)
    (`Widget.RemoveFromParent` (`self.UIForgeWindow`))))

(fn `UserConstructionScript`
  (`parent.UserConstructionScript`))