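; BP_Interactive_Rock is an interactable rock that yields gold when the player interacts with it.
; Each interaction has its Inventory throw one Gold item in the direction of the first player's pawn.
; Overlap with a StaticMeshActor spawns a dust particle effect at the rock's location.
; An unconnected ThrowAllItems call remains in the event graph and never runs.
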(event `self.ReceiveActorBeginOverlap`
  (params (OtherActor :type "Actor Object Reference"))
  (cast `StaticMeshActor` OtherActor)
  (`GameplayStatics.SpawnEmitterAtLocation` "/Game/Environments/Interactables/Interactable_Rock/ParticleSystem/PS_DustEffect.PS_DustEffect" (`self.K2_GetActorLocation`)))

(event `self.BPInteract`
  (params (toolid :type Name))
  (`InventoryComponent.ThrowItemInDirection` (`self.Inventory`) (`self.Gold`) 1 (- (`self.K2_GetActorLocation` (`GameplayStatics.GetPlayerPawn` 0)) (`self.K2_GetActorLocation`))))

(fn `UserConstructionScript`)