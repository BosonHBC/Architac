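; Warehouse building block that stores items and lets the player transfer them to and from their own inventory.
; Opening it creates a slot-grid widget and maps grid offsets to itself and the player pawn.
; Indicator moves past the window edge hand focus to the mapped pawn, and interact transfers the highlighted slot out of whichever inventory has focus.
; The construction script passes the Inventory to the power receiver and consumer components.
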(event `self.OpenWindow`
  (bind _inventory (`self.Inventory`))
  (bind _relationpointers (`self.RelationPointers`))
  ;[1 1 1] Open warehouse UI
  (`BlueprintMapLibrary.Map_Add` (`self.RelationPointers`) (make `IntVector` 0 1) (`GameplayStatics.GetPlayerPawn` 0))
  (`BlueprintMapLibrary.Map_Add` _relationpointers (make `IntVector` 0) self)
  (set `self.copyrelationdata` _relationpointers)
  (bind _returnvalue (`InventoryComponent.GetInventorySlotNum` _inventory))
  (bind _returnvalue_2 (`|CreateWidget` "/Game/UI/WarehouseUI/BP_UI_WarehouseWindow.BP_UI_WarehouseWindow_C" (`GameplayStatics.GetPlayerController` 0) _inventory _returnvalue))
  (bind _output_get (set `self.UIWarehouseWindow` _returnvalue_2))
  (`UserWidget.AddToViewport` _returnvalue_2 0)
  (`UserWidget.AddToViewport` _output_get 0)
  (`/Game/UI/BasicUI/BP_BasicUI_Window.SetUpInitialSlotPosition` _returnvalue_2))

(event `self.CloseWindow`
  ;[1 1 1] Close warehouse UI
  (`Widget.RemoveFromParent` (`self.UIWarehouseWindow`))
  (bind _asbp_venture_player (cast `/Game/Characters/Player/Blueprints/BP_VenturePlayer` (`GameplayStatics.GetPlayerPawn` 0)))
  (`/Game/UI/BasicUI/BP_BasicUI_Window.UnHighlightCurrentSlot` (`/Game/Characters/Player/Blueprints/BP_VenturePlayer.PlayerInventory` _asbp_venture_player)))

(event `self.MoveIndicator`
  (params (direction :type "IntVector Structure") (istheoriginalwindow :type Boolean))
  (bind (_x _y _z) (break `IntVector` (`self.CurrentFocusingWindow`)))
  (bind (_value _returnvalue) (`BlueprintMapLibrary.Map_Find` (`self.copyrelationdata`) (`self.CurrentFocusingWindow`)))
  ;[1 1 1] MoveSlotIndicator
  (if (and (== _x 0) (== _y 0) (== _z 0))
    (bind (_updatedposition _isinthiswindow) (`/Game/UI/BasicUI/BP_BasicUI_Window.MoveSlotIndicator` (`self.UIWarehouseWindow`) direction))
    (if _isinthiswindow
      (set `self.CurrentFocusingWindow` (make `IntVector` 0))
      (else
        (bind (_value_2 _returnvalue_2) (`BlueprintMapLibrary.Map_Find` (`self.copyrelationdata`) _updatedposition))
        (if _returnvalue_2
          (`/Game/UI/BasicUI/BP_BasicUI_Window.UnHighlightCurrentSlot` (`self.UIWarehouseWindow`))
          (set `self.CurrentFocusingWindow` _updatedposition)
          (bind _asventure_pawn (cast `VenturePawn` _value_2))
          (`VenturePawn.FocusThisWindow` _asventure_pawn self))))
    (elif _returnvalue
      (bind _asventure_pawn_2 (cast `VenturePawn` _value))
      (`VenturePawn.MoveUIIndicator` _asventure_pawn_2 direction false))))

(event `self.FocusThisWindow`
  (params (sender :type "Actor Object Reference"))
  ;[1 1 1] Focus to this window
  (set `self.CurrentFocusingWindow` (make `IntVector` 0))
  (`/Game/UI/BasicUI/BP_BasicUI_Window.SetUpInitialSlotPosition` (`self.UIWarehouseWindow`)))

(event `self.ReceiveBeginPlay`
  ;[1 1 1] Set up relation pointer
)

(event `self.InteractWithUI`
  (bind _uiwarehousewindow (`self.UIWarehouseWindow`))
  (bind (_x _y _z) (break `IntVector` (`self.CurrentFocusingWindow`)))
  ;[1 1 1] InteractWithUI
  (if (and (== _x 0) (== _y 0) (== _z 0))
    (bind _data (`/Game/UI/BasicUI/BP_BasicUI_Window.GetInventoryDataInCurrentSlot` _uiwarehousewindow))
    (bind _asventure_pawn (cast `VenturePawn` (`GameplayStatics.GetPlayerPawn` 0)))
    (bind (_itemid _itempickup _name _action _amount) (break `InventoryItem` _data))
    (`InventoryUtility.TransferItemOnlyBySrcSlot` (`self.Inventory`) (`VenturePawn.InventoryComp` _asventure_pawn) _itemid _amount (`/Game/UI/BasicUI/BP_BasicUI_Window.CurrentSlotPosition` _uiwarehousewindow))
    (else
      (bind _asbp_venture_player (cast `/Game/Characters/Player/Blueprints/BP_VenturePlayer` (`GameplayStatics.GetPlayerPawn` 0)))
      (bind _playerinventory (`/Game/Characters/Player/Blueprints/BP_VenturePlayer.PlayerInventory` _asbp_venture_player))
      (bind _data_2 (`/Game/UI/BasicUI/BP_BasicUI_Window.GetInventoryDataInCurrentSlot` _playerinventory))
      (bind (_itemid_2 _itempickup_2 _name_2 _action_2 _amount_2) (break `InventoryItem` _data_2))
      (`InventoryUtility.TransferItemOnlyBySrcSlot` (`VenturePawn.InventoryComp` _asbp_venture_player) (`self.Inventory`) _itemid_2 _amount_2 (`/Game/UI/BasicUI/BP_BasicUI_Window.CurrentSlotPosition` _playerinventory)))))

(fn `UserConstructionScript`
  (bind _inventory (`self.Inventory`))
  (`ReceiverComponent.SetReceiverProperties` (`self.PowerReceiver`) _inventory)
  (`ConsumptionComponent.SetConsumptionProperties` (`self.PowerConsumer`) _inventory))