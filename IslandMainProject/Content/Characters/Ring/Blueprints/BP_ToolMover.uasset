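; BP_ToolMover drives the Ring character's tool readying, switching and use, including a three-step attack combo.
; Its events write state, tool name and combo index into BP_RingAnimBP, and tool use plays harpoon or pickaxe swing sounds through the game mode's AudioManager.
; Finishing a use advances the combo, which resets after the third step, a tool switch or an idle delay.
; Launch reuses KnockBackActor to push the player forward by combo step.
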(event `self.ReceiveBeginPlay`
  (bind _asbp_ring_anim_bp (cast `/Game/Characters/Ring/Animation/BP_RingAnimBP` (`SkeletalMeshComponent.GetAnimInstance` (`self.SuperMesh`))))
  (set `self.AnimationBP` _asbp_ring_anim_bp)
  (bind _asbp_game_mode (cast `/Game/Base/BP_GameMode` (`GameplayStatics.GetGameMode`)))
  (set `self.AudioManager` (`/Game/Base/BP_GameMode.AudioManager` _asbp_game_mode)))

(event `self.BPGetToolReady`
  (params (toolID :type Name))
  (bind _animationbp (`self.AnimationBP`))
  (set `/Game/Characters/Ring/Animation/BP_RingAnimBP.m_Ready` true _animationbp)
  (set `/Game/Characters/Ring/Animation/BP_RingAnimBP.m_IncomeName` toolID _animationbp))

(event `self.BPDisconnectTool`
  (bind _animationbp (`self.AnimationBP`))
  (set `/Game/Characters/Ring/Animation/BP_RingAnimBP.m_Ready` false _animationbp)
  (set `/Game/Characters/Ring/Animation/BP_RingAnimBP.m_IncomeName` "None" _animationbp))

(event `self.BPUseTool`
  (params (toolID :type Name))
  (bind _animationbp (`self.AnimationBP`))
  (bind _audiomanager (`self.AudioManager`))
  (set `/Game/Characters/Ring/Animation/BP_RingAnimBP.m_Using` true _animationbp)
  (bind _output_get (set `/Game/Characters/Ring/Animation/BP_RingAnimBP.m_IncomeName` toolID _animationbp))
  (bind _output_get_2 (set `/Game/Characters/Ring/Animation/BP_RingAnimBP.comatCombo` (`self.combatCombo`) _animationbp))
  (`KismetSystemLibrary.PrintString` (`KismetStringLibrary.Concat_StrStr` "Current Combo: " (`KismetStringLibrary.Conv_IntToString` _output_get_2)))
  (`/Engine/EditorBlueprintResources/StandardMacros.IsValid` _audiomanager
    (:`Is Valid`
      (switch `name` _output_get
        (:`Harpoon`
          (`AudioManagerComponent.Play` _audiomanager "PlayerHarpoonSwing" (0.0 0.0 0.0)))
        (:`Pickaxe`
          (`AudioManagerComponent.Play` _audiomanager "PlayerAxeSwing" (0.0 0.0 0.0)))))))

(event `self.BPUseToolFinish`
  (bind _result (`/Engine/EditorBlueprintResources/StandardMacros.IncrementInt` (`self.combatCombo`))
    (:`  `
      (if (>= _result 3)
        (`KismetSystemLibrary.PrintString` "Reset Combo  because combo more than 3")
        (`self.ResetCombo` :!label _label)
        (else
          (`KismetSystemLibrary.PrintString` "Use Tool Finish")
          (`KismetSystemLibrary.Delay` (`self.delayToReset`))
          (if (not (`/Game/Characters/Ring/Animation/BP_RingAnimBP.m_Using` (`self.AnimationBP`)))
            (`KismetSystemLibrary.PrintString` "Reset Combo because not attack anymore")
            (goto _label)))))))

(event `self.BPSwitchTool`
  (params (toolID :type Name))
  (bind _animationbp (`self.AnimationBP`))
  (set `/Game/Characters/Ring/Animation/BP_RingAnimBP.m_SwitchingItem` true _animationbp)
  (set `/Game/Characters/Ring/Animation/BP_RingAnimBP.m_IncomeName` toolID _animationbp)
  (set `self.combatCombo` 0))

(fn `Launch`
  (bind _m_venturepawn (`self.m_venturePawn`))
  (switch `int` (`self.combatCombo`)
    (:`0`
      (set `self.LaunchForce` 0.0))
    (:`1`
      (set `self.LaunchForce` 120.0))
    (:`2`
      (set `self.LaunchForce` 45.0)))
  (`StaticFunctionLibary.KnockBackActor` _m_venturepawn (`self.GetActorForwardVector` _m_venturepawn) (`self.LaunchForce`) 0.2))

(fn `ResetCombo`
  (set `self.combatCombo` 0))

(fn `UserConstructionScript`)